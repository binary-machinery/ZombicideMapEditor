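; BP_EditorView sets up the tile palette UI for an editor view, displaying the available tile sprites on screen.
; On BeginPlay it adds a WBP_TileList widget to the viewport and shows the first player's mouse cursor.
; It then creates a WBP_TileListItem for each entry in TileSprites, sets its image brush from that sprite and adds it to the list's wrap box.
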(event `self.ReceiveBeginPlay`
  (bind _returnvalue (`|CreateWidget` "/Game/UI/WBP_TileList.WBP_TileList_C"))
  (`UserWidget.AddToViewport` _returnvalue 0)
  (set `PlayerController.bShowMouseCursor` true (`GameplayStatics.GetPlayerController` 0))
  (for _array_element (`self.TileSprites`)
    (bind _returnvalue_2 (`|CreateWidget` "/Game/UI/WBP_TileListItem.WBP_TileListItem_C"))
    (`Image.SetBrush` (`/Game/UI/WBP_TileListItem.Sprite` _returnvalue_2) (`PaperSpriteBlueprintLibrary.MakeBrushFromSprite` _array_element))
    (`WrapBox.AddChildToWrapBox` (`/Game/UI/WBP_TileList.TileListContainer` _returnvalue) _returnvalue_2)))

(fn `UserConstructionScript`)